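; Enemy NPC that shoots at the third-person player while they are inside its Deteccion volume.
; Overlap starts a looping Disparar timer and turns the actor toward the player every Tick; leaving clears both.
; Each shot line-traces from PuntoDisparo on Visibility, applying effects and calling RecibirDanho only if the player is hit.
; JugadorMuerto stops firing; EnemigoEliminado also plays a death animation, then destroys the actor after a delay.
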(event `self.ReceiveBeginPlay`
  (`parent.ReceiveBeginPlay`))

(event `Enemigo Eliminado`
  (`SkeletalMeshComponent.PlayAnimation` (`self.Mesh`) "/Game/MisCosas/Importado/Animaciones/Death.Death" false)
  (`KismetSystemLibrary.K2_ClearTimer` null "Disparar")
  (`KismetSystemLibrary.Delay` 4.0)
  (`self.K2_DestroyActor`))

(event `self.Deteccion.OnComponentBeginOverlap`
  (params (OverlappedComponent :type "PrimitiveComponent Object Reference") (OtherActor :type "Actor Object Reference") (OtherComp :type "PrimitiveComponent Object Reference") (OtherBodyIndex :type Integer) (bFromSweep :type Boolean) (SweepResult :type "HitResult Structure (by ref)"))
  (bind _asbp_third_person_character (cast `/Game/MisCosas/BP_ThirdPersonCharacter` OtherActor))
  (set `self.Jugador` _asbp_third_person_character)
  (`KismetSystemLibrary.K2_SetTimer` null "Disparar" (`self.TiempoEntreDisparos`) true)
  (set `self.JugadorVisto` true))

(event `self.ReceiveTick`
  (params (DeltaSeconds :type "Float (single-precision)"))
  (`parent.ReceiveTick` DeltaSeconds)
  (if (`self.JugadorVisto`)
    (`self.Rotar`)))

(event `self.Deteccion.OnComponentEndOverlap`
  (params (OverlappedComponent :type "PrimitiveComponent Object Reference") (OtherActor :type "Actor Object Reference") (OtherComp :type "PrimitiveComponent Object Reference") (OtherBodyIndex :type Integer))
  (cast `/Game/MisCosas/BP_ThirdPersonCharacter` OtherActor)
  (`KismetSystemLibrary.K2_ClearTimer` null "Disparar")
  (set `self.JugadorVisto` false))

(event `Jugador Muerto`
  (`KismetSystemLibrary.K2_ClearTimer` null "Disparar"))

(event `Rotar`
  (`self.K2_SetActorRotation` (`KismetMathLibrary.FindLookAtRotation` (`SceneComponent.K2_GetComponentLocation` (`self.Punto disparo`)) (`self.K2_GetActorLocation` (`self.Jugador`)))))

(event `Disparar`
  (`/Engine/EditorBlueprintResources/StandardMacros.IsValid` (`self.Jugador`)
    (:`Is Valid`
      (`self.Comprobar visibilidad`))))

(event `Comprobar visibilidad`
  (bind _outhit (`KismetSystemLibrary.LineTraceSingle` (`SceneComponent.K2_GetComponentLocation` (`self.Punto disparo`)) (+ (`self.K2_GetActorLocation` (`self.Jugador`)) (0.0 0.0 60.0)) "TraceTypeQuery1"))
  (if (== (`.HitActor` (`GameplayStatics.BreakHitResult` _outhit)) (`self.Jugador`))
    (`self.Efectos de Disparo`)
    (`/Game/MisCosas/BP_ThirdPersonCharacter.Recibir danho` (`self.Jugador`))))

(event `Efectos de Disparo`
  (bind _punto_disparo (`self.Punto disparo`))
  (bind _returnvalue (`SceneComponent.K2_GetComponentLocation` _punto_disparo))
  (`GameplayStatics.SpawnEmitterAtLocation` "/Game/StarterContent/Particles/P_Explosion.P_Explosion" _returnvalue (`SceneComponent.K2_GetComponentRotation` _punto_disparo) (0.05 0.05 0.05))
  (`GameplayStatics.PlaySoundAtLocation` "/Game/StarterContent/Audio/Explosion02.Explosion02" _returnvalue (struct) 1.0 1.0 0.0 null null null null))

(fn `UserConstructionScript`
  (`parent.UserConstructionScript`))